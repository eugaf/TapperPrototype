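; A Paper2D enemy character, apparently a basic side-scroller AI, that switches between walk and idle flipbooks based on its velocity.
; BeginPlay applies a single negative-X force through CharacterMovement, and any capsule hit stops movement immediately.
; Tick refreshes the animation every frame.
; Unconnected nodes for sprite replication and movement input never run.
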(event OnComponentHit(CapsuleComponent)
  (params (HitComponent :type Primitive%20Component%20Object%20Reference) (OtherActor :type Actor%20Object%20Reference) (OtherComp :type Primitive%20Component%20Object%20Reference) (NormalImpulse :type Vector :default "0, 0, 0") (Hit :type Hit%20Result%20Structure%20%28by%20ref%29))
  ;[1 1 1] Handle movement
  (Components|Movement|StopMovementImmediately (Variables|Character|GetCharacterMovement)))

(event Custom|UpdateAnimation
  ;[1 1 1] Handle Animation
  (Sprite|SetFlipbook (Variables|Default|GetSprite) (select (> (Math|Vector|VectorLength (Transformation|GetVelocity)) 0.0) "/Game/Sprites/Enemies/e1_walk.e1_walk" "/Game/Sprites/Enemies/e1_idle.e1_idle")))

(event EventTick
  (params (DeltaSeconds :type Float%20%28single-precision%29))
  ;[1 1 1] Tick - Updates animation
  (CallFunction|UpdateAnimation))

(event EventBeginPlay
  ;[1 1 1] Handle movement
  (Physics|AddForce (Variables|Character|GetCharacterMovement) "-1.000000, 0, 0"))

(fn ConstructionScript)