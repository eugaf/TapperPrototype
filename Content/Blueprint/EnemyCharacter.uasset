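; EnemyCharacter is a 2D flipbook enemy character that constantly walks toward negative world X.
; Each tick it adds that movement input, then updates sprite facing and animation.
; Facing flips the sprite's yaw based on IsMovingRight, which this file never sets.
; Animation picks Walk or Idle from velocity, and SetFlipBook stores that state and swaps the matching flipbook.
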(event Custom|AnimationUpdate
  ;[1 1 1] Idle and Run Controller
  (CallFunction|SetFlipBook (select (> (Math|Vector|VectorLength (Transformation|GetVelocity)) 0.0) "NewEnumerator1" "NewEnumerator0")))

(event Custom|Direction
  ;[1 1 1] Direction
  (Transformation|SetRelativeRotation (Variables|Default|GetSprite) (Math|Rotator|MakeRotator 0.0 0.0 (Math|Float|SelectFloat 0.0 1.8e+02 (Variables|Default|GetisMovingRight))) false false))

(event EventTick
  (params (DeltaSeconds :type Float%20%28single-precision%29))
  ;[1 1 1] Direction
  (Pawn|Input|AddMovementInput "-1.000000, 0, 0" 1.0 false)
  (CallFunction|Direction)
  (CallFunction|AnimationUpdate))

(fn ConstructionScript)

(fn SetFlipBook
  (params (NextState :type AnimStates2D%20Enum))
  (Variables|Default|SetcurrentState NextState)
  (Sprite|SetFlipbook (Variables|Default|GetSprite) (Utilities|Select :Index (Variables|Default|GetcurrentState) :NewEnumerator0 (Variables|Default|GetFB_Idle) :NewEnumerator1 (Variables|Default|GetFB_Walk))))