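; A 2D side-scrolling Paper2D character that moves along world X from the MoveRight axis and remembers its last input direction.
; Each tick it turns the controller yaw to face its X velocity, falling back to the remembered direction when still.
; Tick also picks Idle or Walk from velocity magnitude, and SetFlipBook stores that state and applies the matching flipbook to the sprite.
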(event Custom|AnimationUpdate
  ;[1 1 1] Idle and Run Controller
  (CallFunction|SetFlipBook (select (> (Math|Vector|VectorLength (Transformation|GetVelocity)) 0.0) "NewEnumerator1" "NewEnumerator0")))

(event Custom|Direction
  (bind _returnvalue (Pawn|GetController))
  ;[1 1 1] Direction
  (Math|Float|CompareFloat (.x (Transformation|GetVelocity)) 0.0
    (:>
      (Pawn|SetControlRotation _returnvalue (Math|Rotator|MakeRotator 0.0 0.0 0.0) :!label _label))
    (:==
      (if (Variables|Default|GetisMovingRight)
        (goto _label)
        (else
          (Pawn|SetControlRotation _returnvalue (Math|Rotator|MakeRotator 0.0 0.0 1.8e+02) :!label _label_2))))
    (:<
      (goto _label_2))))

(event EventBeginPlay)

(event EventTick
  (params (DeltaSeconds :type Float%20%28single-precision%29))
  (CallFunction|Direction)
  (CallFunction|AnimationUpdate))

(event Input|AxisEvents|InputAxisMoveRight
  (params (AxisValue :type Float%20%28single-precision%29))
  ;[1 1 1] Move Input
  (Math|Float|CompareFloat AxisValue 0.0
    (:>
      (Variables|Default|SetisMovingRight true))
    (:<
      (Variables|Default|SetisMovingRight false)))
  (Pawn|Input|AddMovementInput "1.000000, 0, 0" AxisValue false))

(fn ConstructionScript)

(fn SetFlipBook
  (params (NextState :type AnimStates2D%20Enum))
  (Variables|Default|SetcurrentState NextState)
  (Sprite|SetFlipbook (Variables|Default|GetSprite) (Utilities|Select :Index (Variables|Default|GetcurrentState) :NewEnumerator0 (Variables|Default|GetFB_Idle) :NewEnumerator1 (Variables|Default|GetFB_Walk))))